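; BP_Player is the player in GeometryCatcher, moving sideways and toggling the pause menu.
; The MoveRight axis adds movement input scaled by MaxSpeed, and Tick consumes that vector as a swept, frame-time-scaled actor offset.
; BeginPlay creates the Pause widget for player controller index 1 and adds it to the viewport.
; The P key toggles the game's paused state along with that widget's visibility.
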(event EventBeginPlay
  (bind _returnvalue (UserInterface|CreateWidget "/Game/GeometryCatcher/Blueprints/Pause.Pause_C" (Game|GetPlayerController 1)))
  (UserInterface|Viewport|AddtoViewport _returnvalue 0))

(event EventTick
  (params (DeltaSeconds :type Float%20%28single-precision%29))
  (bind _returnvalue (Class|Pawn|ConsumeMovementInputVector))
  (Transformation|AddActorLocalOffset (* _returnvalue DeltaSeconds) true false))

(event Input|AxisEvents|InputAxisMoveRight
  (params (AxisValue :type Float%20%28single-precision%29))
  (Pawn|Input|AddMovementInput (Transformation|GetActorRightVector) (* AxisValue (Variables|Default|GetMaxSpeed)) false))

(event Input|KeyboardEvents|P
  (params (Key :type Key%20Structure :default "None"))
  (:Pressed
    (if (Game|IsGamePaused)
      (Widget|SetVisibility (stale EventBeginPlay _returnvalue) "Hidden")
      (Game|SetGamePaused false)
      (else
        (Widget|SetVisibility (stale EventBeginPlay _returnvalue) "Visible")
        (Game|SetGamePaused true)))))

(fn ConstructionScript)